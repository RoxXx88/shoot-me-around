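; Projectile bullet actor for the ShootMeAround game that damages players on hit and counts its bounces off other objects.
; On hitting an SMA_Character it applies PlayerDamage, switches off its collision, mesh, movement and particles, then destroys itself after a short delay.
; Any other hit increments a bounce counter and compares it to NumberOfBounces, but nothing follows that check.
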(event Collision|EventHit
  (params (MyComp :type Primitive%20Component%20Object%20Reference) (Other :type Actor%20Object%20Reference) (OtherComp :type Primitive%20Component%20Object%20Reference) (bSelfMoved :type Boolean) (HitLocation :type Vector :default "0, 0, 0") (HitNormal :type Vector :default "0, 0, 0") (NormalImpulse :type Vector :default "0, 0, 0") (Hit :type Hit%20Result%20Structure%20%28by%20ref%29))
  (bind _collision (Variables|Default|GetCollision))
  (bind _mesh (Variables|Default|GetMesh))
  ;[1 1 1] If bullet hit a Player
  (bind _assma_character (Utilities|Casting|CastToSMA_Character Other)
    (:then
      (Game|Damage|ApplyDamage _assma_character (Variables|Default|GetPlayerDamage) 0 0)
      ;[1 1 1] Disable and Deactive the component of Actor, before destroy it
      (Collision|SetCollisionEnabled _collision "NoCollision")
      (Components|Activation|Deactivate _collision)
      (Components|Activation|Deactivate _mesh)
      (Rendering|SetVisibility _mesh false false)
      (Components|Activation|Deactivate (Variables|Default|GetProjectileMovement))
      (Components|Activation|Deactivate (Variables|Default|GetParticleSystem))
      ;[1 1 1] Wait before destroy actor
      (Utilities|FlowControl|Delay 3.0)
      (Actor|DestroyActor))
    (:CastFailed
      ;[1 1 1] If the bullet hit an object
      (Math|Integer|IncrementInt (Variables|Default|GetBouncesCounter)
        (:%20%20
          (if (>= (Variables|Default|GetBouncesCounter) (Variables|Default|GetNumberOfBounces))
            _))))))

(fn ConstructionScript)